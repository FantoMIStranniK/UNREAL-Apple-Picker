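; Player-controlled basket for an apple picker game that slides along a fixed line to catch apples.
; The BasketAxis input sets a direction, which Tick integrates with Speed into a clamped 0–1 progress value that lerps the swept actor location between StartPoint and EndPoint.
; Any actor overlapping the basket mesh is destroyed without a type check, adding score through the cached ApplePickerState and playing the apple sound.
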(event `self.ReceiveBeginPlay`
  (bind _asapple_picker_state (cast `/Game/Gamemode/ApplePickerState` (`GameplayStatics.GetGameState`)))
  (set `self.PickerState` _asapple_picker_state))

(event `self.ReceiveTick`
  (params (DeltaSeconds :type "Float (single-precision)"))
  (`self.GetProgress` DeltaSeconds)
  (`self.Move`))

(event `InputAxis|BasketAxis`
  (params (AxisValue :type "Float (single-precision)"))
  (set `self.Direction` AxisValue))

(event `self.BasketMesh.OnComponentBeginOverlap`
  (params (OverlappedComponent :type "PrimitiveComponent Object Reference") (OtherActor :type "Actor Object Reference") (OtherComp :type "PrimitiveComponent Object Reference") (OtherBodyIndex :type Integer) (bFromSweep :type Boolean) (SweepResult :type "HitResult Structure (by ref)"))
  (`self.K2_DestroyActor` OtherActor)
  (`/Game/Gamemode/ApplePickerState.Add Score` (`self.PickerState`))
  (`AudioSubsystem.PlaySound` (subsystem `AudioSubsystem`) "/Game/Audio/AppleSound.AppleSound" 0.2))

(fn `GetProgress`
  (params (DeltaTime :type "Float (double-precision)"))
  (set `self.Progress` (`KismetMathLibrary.FClamp` (+ (* (`self.Speed`) DeltaTime (`self.Direction`)) (`self.Progress`))))
  (return))

(fn `Move`
  (`self.K2_SetActorLocation` (`KismetMathLibrary.VLerp` (`self.StartPoint`) (`self.EndPoint`) (`self.Progress`)) true))

(fn `UserConstructionScript`)